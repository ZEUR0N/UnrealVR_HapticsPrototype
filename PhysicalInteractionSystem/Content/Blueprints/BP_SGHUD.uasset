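; BP_SGHUD is a HUD Blueprint that shows an on-screen key legend for a SenseGlove (SG) glove test or demo.
; On DrawHUD, if the DrawHUD flag is set, it draws a title and a fixed column of text lines using shared color, font and X-position variables.
; The lines describe keys for library versions, glove connection, haptic commands and debug virtual hand drawing; the file itself handles no input.
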(event `self.ReceiveDrawHUD`
  (params (SizeX :type Integer) (SizeY :type Integer))
  (if (`self.Draw HUD`)
    (`self.DrawText` "Press any of the following keys on the keyboard:" (`self.Draw Color`) (`self.Draw Location X`) 100.0 "/Game/Fonts/Font_Title.Font_Title")
    (`self.DrawText` "0): Toggle this message off/on" (`self.Draw Color`) (`self.Draw Location X`) 200.0 "/Game/Fonts/Font_Keys.Font_Keys")
    (`self.DrawText` "1: Get SGConnect/SGCore underlying libraries versions" (`self.Draw Color`) (`self.Draw Location X`) 250.0 "/Game/Fonts/Font_Keys.Font_Keys")
    (`self.DrawText` "2: Check whether a glove is connected or not; if connected, initialize it and show some extra info" (`self.Draw Color`) (`self.Draw Location X`) 300.0 "/Game/Fonts/Font_Keys.Font_Keys")
    (`self.DrawText` "3: Send or stop a Buzz haptic command" (`self.Draw Color`) (`self.Draw Location X`) 350.0 "/Game/Fonts/Font_Keys.Font_Keys")
    (`self.DrawText` "4: Send or stop a Force-feedback haptic command" (`self.Draw Color`) (`self.Draw Location X`) 400.0 "/Game/Fonts/Font_Keys.Font_Keys")
    (`self.DrawText` "5: Send or stop a Thumper haptic command" (`self.Draw Color`) (`self.Draw Location X`) 450.0 "/Game/Fonts/Font_Keys.Font_Keys")
    (`self.DrawText` "6: Force stop all haptics if any" (`self.Draw Color`) (`self.Draw Location X`) 500.0 "/Game/Fonts/Font_Keys.Font_Keys")
    (`self.DrawText` "7: Read and visualize the glove data as a debug virtual hand using cubic joints" (`self.Draw Color`) (`self.Draw Location X`) 550.0 "/Game/Fonts/Font_Keys.Font_Keys")
    (`self.DrawText` "8: Read and visualize the glove data as a debug virtual hand using gizmo joints" (`self.Draw Color`) (`self.Draw Location X`) 600.0 "/Game/Fonts/Font_Keys.Font_Keys")
    (`self.DrawText` "9:Stop drawing the debug virtual hand" (`self.Draw Color`) (`self.Draw Location X`) 650.0 "/Game/Fonts/Font_Keys.Font_Keys")))

(fn `UserConstructionScript`)